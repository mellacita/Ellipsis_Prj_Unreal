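; Interactable old radio actor that toggles its music on and off when triggered through an interact interface call.
; Interaction branches on an IsRadioOn flag, and both paths play a sound at the radio mesh's location.
; Turning on waits briefly before starting the OldRadioMusic audio and setting the flag, while turning off stops it and clears the flag immediately.
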(event `/Game/Data/BPI_Interact.BPI_Interact`
  ;[1 1 1] Event BP Interface Call Function
  (`self.Toggle Radio ON OFF`))

(event `Toggle Radio ON OFF`
  ;[1 1 1] Toggle ON / OFF
  (if (`self.Is Radio On?`)
    (`self.TurnRadioOff`)
    (else
      (`self.TurnRadioOn`))))

(event `TurnRadioOn`
  ;[1 1 1] Turn Radio ON
  (`GameplayStatics.PlaySoundAtLocation` "/Game/Audio/SoundCue/OldRadioMusic.OldRadioMusic" (`SceneComponent.K2_GetComponentLocation` (`self.SM_OldRadio`)) (struct) 1.0 1.0 0.0 null null null null)
  (`KismetSystemLibrary.Delay` 1.0)
  (`AudioComponent.Play` (`self.OldRadioMusic`) 0.0)
  (set `self.Is Radio On?` true))

(event `TurnRadioOff`
  ;[1 1 1] Turn Radio OFF
  (`GameplayStatics.PlaySoundAtLocation` "/Game/Audio/SoundCue/OldRadioMusic.OldRadioMusic" (`SceneComponent.K2_GetComponentLocation` (`self.SM_OldRadio`)) (struct) 1.0 1.0 0.0 null null null null)
  (`AudioComponent.Stop` (`self.OldRadioMusic`))
  (set `self.Is Radio On?` false))

(fn `UserConstructionScript`)